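; Behavior tree task that repeatedly tells the AI to set its weapon while it has an enemy target.
; On execute it casts the owner to BP_AI_Controller and starts a looping one-second timer that calls the controller's SetWeapon.
; Each tick of that timer checks the blackboard enemy key, and once no valid enemy remains it clears the timer and finishes successfully.
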(event `self.ReceiveExecuteAI`
  (params (OwnerController :type "AIController Object Reference") (ControlledPawn :type "Pawn Object Reference"))
  (bind _asbp_ai_controller (cast `/Game/Blueprints/AI/BP_AI_Controller` OwnerController))
  (bind _returnvalue (`KismetSystemLibrary.K2_SetTimerDelegate` (delegate `SetWeapon`) 1.0 true 1.0))
  (set `self.Timer` _returnvalue))

(event `SetWeapon`
  (`/Game/Blueprints/AI/BP_AI_Controller.SetWeapon` (stale `self.ReceiveExecuteAI` _asbp_ai_controller))
  (bind _returnvalue (`AIBlueprintHelperLibrary.GetBlackboard` (stale `self.ReceiveExecuteAI` _asbp_ai_controller)))
  (`/Engine/EditorBlueprintResources/StandardMacros.IsValid` _returnvalue
    (:`Is Valid`
      (`/Engine/EditorBlueprintResources/StandardMacros.IsValid` (`BlackboardComponent.GetValueAsObject` _returnvalue (`self.EnemyActorKey`))
        (:`Is Not Valid`
          (`KismetSystemLibrary.K2_ClearAndInvalidateTimerHandle` (`self.Timer`))
          (`self.FinishExecute` true))))))