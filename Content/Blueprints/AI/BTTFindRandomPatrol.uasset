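; Behavior Tree task that picks a random patrol destination for a BP_AI_Character.
; It sets the character to walk speed, then stores a random reachable point within the patrol radius in a Blackboard vector key, falling back to the pawn's current location.
; The reachability check and the stored point come from separate random queries.
; The task succeeds after writing the key and fails if the pawn cast fails.
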(event `self.ReceiveExecuteAI`
  (params (OwnerController :type "AIController Object Reference") (ControlledPawn :type "Pawn Object Reference"))
  (bind _returnvalue (`Actor.K2_GetActorLocation` ControlledPawn))
  (bind _key_name (`self.Key Name`))
  (bind (_randomlocation _returnvalue_2) (`NavigationSystemV1.K2_GetRandomReachablePointInRadius` _returnvalue (`self.Patrol Radius`) null null))
  (bind _asbp_ai_character (cast `/Game/Blueprints/AI/BP_AI_Character` ControlledPawn)
    (:`then`
      (`/Game/Blueprints/AI/BP_AI_Character.UpdateSpeed` _asbp_ai_character (`self.Walk Speed`))
      (if _returnvalue_2
        (bind _returnvalue_3 (`AIBlueprintHelperLibrary.GetBlackboard` _asbp_ai_character))
        (`BlackboardComponent.SetValueAsVector` _returnvalue_3 _key_name _randomlocation)
        (else
          (`BlackboardComponent.SetValueAsVector` _returnvalue_3 _key_name _returnvalue)))
      (`self.FinishExecute` true))
    (:`CastFailed`
      (`self.FinishExecute` false))))