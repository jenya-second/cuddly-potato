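; Behavior Tree task that keeps moving the AI pawn to a fight spot while it has an enemy.
; A looping half-second timer gets the spot from BP_AI_Controller and reissues AIMoveTo.
; Without waiting for arrival, each tick writes the spot to PatrolLocationKey, then clears the timer and finishes successfully if EnemyActorKey holds no valid actor.
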(event `self.ReceiveExecuteAI`
  (params (OwnerController :type "AIController Object Reference") (ControlledPawn :type "Pawn Object Reference"))
  (bind _asbp_ai_controller (cast `/Game/Blueprints/AI/BP_AI_Controller` OwnerController))
  (bind _returnvalue (`KismetSystemLibrary.K2_SetTimerDelegate` (delegate `Find Location`) 0.5 true))
  (set `self.Timer` _returnvalue))

(event `Find Location`
  (bind _location (`/Game/Blueprints/AI/BP_AI_Controller.GetFightSpot` (stale `self.ReceiveExecuteAI` _asbp_ai_controller)))
  (`|AIMoveTo` (stale `self.ReceiveExecuteAI` ControlledPawn) _location null
    (:`then`
      (bind _returnvalue (`AIBlueprintHelperLibrary.GetBlackboard` (stale `self.ReceiveExecuteAI` _asbp_ai_controller)))
      (`BlackboardComponent.SetValueAsVector` _returnvalue (`self.PatrolLocationKey`) _location)
      (`/Engine/EditorBlueprintResources/StandardMacros.IsValid` (`BlackboardComponent.GetValueAsObject` _returnvalue (`self.EnemyActorKey`))
        (:`Is Not Valid`
          (`KismetSystemLibrary.K2_ClearAndInvalidateTimerHandle` (`self.Timer`))
          (`self.FinishExecute` true))))))