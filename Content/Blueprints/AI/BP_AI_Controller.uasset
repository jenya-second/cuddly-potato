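; AI controller for team-based combat bots that runs a behavior tree and tracks perceived enemies on the blackboard, clearing them on a timer.
; Each tick it smoothly turns toward the enemy and sphere-traces from the camera to set the can-shoot key.
; GetFightSpot samples a ring around the enemy for the cheapest path.
; SetWeapon and SetBullet use utility scores from match-state coefficients, weighing distance, with bullet affinity for weapons and health/ammo for bullets.
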(event `self.ReceiveBeginPlay`)

(event `self.ReceiveTick`
  (params (DeltaSeconds :type "Float (single-precision)"))
  (`self.SetFocal` DeltaSeconds)
  (`self.CanShoot`))

(event `self.ReceivePossess`
  (params (PossessedPawn :type "Pawn Object Reference"))
  (bind _returnvalue (`self.RunBehaviorTree` "/Game/Blueprints/AI/AITree.AITree"))
  (if _returnvalue
    (`self.Init`)))

(event `self.AIPerception.OnTargetPerceptionUpdated`
  (params (Actor :type "Actor Object Reference") (Stimulus :type "AIStimulus Structure"))
  (bind _asdefault_character (cast `DefaultCharacter` Actor))
  (bind _asdefault_player_state (cast `DefaultPlayerState` (`Pawn.PlayerState` _asdefault_character)))
  (bind _asdefault_player_state_2 (cast `DefaultPlayerState` (`self.PlayerState`)))
  (if (== (`DefaultCharacter.CurrentHealth` _asdefault_character) 0.0)
    _
    (elif (and (!= (`DefaultPlayerState.Team` _asdefault_player_state_2) (`DefaultPlayerState.Team` _asdefault_player_state)) (`.bSuccessfullySensed` (break `AIStimulus` Stimulus)))
      (`KismetSystemLibrary.K2_ClearAndInvalidateTimerHandle` (`self.Enemy Timer`))
      (`/Engine/EditorBlueprintResources/StandardMacros.IsValid` (`BlackboardComponent.GetValueAsObject` (`self.Blackboard`) (`self.EnemyActorKey`))
        (:`Is Not Valid`
          (`BlackboardComponent.SetValueAsObject` (`self.Blackboard`) (`self.EnemyActorKey`) Actor)))
      (else
        (bind _returnvalue (`KismetSystemLibrary.K2_SetTimerDelegate` (delegate `Enemy`) (`self.Time`)))
        (set `self.Enemy Timer` _returnvalue)))))

(event `Enemy`
  (`BlackboardComponent.SetValueAsObject` (`self.Blackboard`) (`self.EnemyActorKey`) null))

(fn `CanShoot`
  (bind _returnvalue (`self.K2_GetPawn`))
  (bind _returnvalue_2 (`AIBlueprintHelperLibrary.GetBlackboard` null))
  (bind _canshootkey (`self.CanShootKey`))
  (`/Engine/EditorBlueprintResources/StandardMacros.IsValid` _returnvalue_2
    (:`Is Valid`
      (`/Engine/EditorBlueprintResources/StandardMacros.IsValid` _returnvalue
        (:`Is Valid`
          (bind _asdefault_character (cast `DefaultCharacter` _returnvalue)
            (:`then`
              (bind _weaponmanager (`DefaultCharacter.WeaponManager` _asdefault_character))
              (bind _output (`|GetArrayItem` (`WeaponManagerComponent.Weapons` _weaponmanager) (`WeaponManagerComponent.IndexWeapon` _weaponmanager)))
              (`/Engine/EditorBlueprintResources/StandardMacros.IsValid` _output
                (:`Is Valid`
                  (bind _camera (`DefaultCharacter.Camera` _asdefault_character))
                  (bind _returnvalue_3 (`SceneComponent.K2_GetComponentLocation` _camera))
                  (bind (_outhit _returnvalue_4) (`KismetSystemLibrary.SphereTraceSingle` _returnvalue_3 (+ (* (`SceneComponent.GetForwardVector` _camera) (`DefaultWeapon.TargetDistance` _output)) _returnvalue_3) (`DefaultWeapon.CheckRadius` _output) "TraceTypeQuery2" false (`|MakeArray` _asdefault_character :!type "Actor Object Reference") "ForOneFrame"))
                  (if _returnvalue_4
                    (bind _asdefault_character_2 (cast `DefaultCharacter` (`.HitActor` (`GameplayStatics.BreakHitResult` _outhit))))
                    (bind _asdefault_player_state (cast `DefaultPlayerState` (`Pawn.PlayerState` _asdefault_character_2)))
                    (bind _asdefault_player_state_2 (cast `DefaultPlayerState` (`Pawn.PlayerState` _asdefault_character)))
                    (`BlackboardComponent.SetValueAsBool` _returnvalue_2 _canshootkey (and (`DefaultWeapon.CanFire` _output) (!= (`DefaultPlayerState.Team` _asdefault_player_state_2) (`DefaultPlayerState.Team` _asdefault_player_state))))))))
            (:`CastFailed`
              (`BlackboardComponent.SetValueAsBool` _returnvalue_2 _canshootkey false :!label _label))))
        (:`Is Not Valid`
          (goto _label))))))

(fn `GetFightSpot`
  (returns (Location :type "Vector Structure"))
  (locals (Loc :type "Vector Structure") (`Path cost` :type "Float (double-precision)" :default 100000000.0))
  (bind _asdefault_character (cast `DefaultCharacter` (`BlackboardComponent.GetValueAsObject` (`self.Blackboard`) (`self.EnemyActorKey`))))
  (for _index (range 21)
    (bind _returnvalue (+ (`self.K2_GetActorLocation` _asdefault_character) (`KismetMathLibrary.GreaterGreater_VectorRotator` (* (`KismetMathLibrary.Vector_Right`) (`self.TargetDistance`)) (`KismetMathLibrary.MakeRotator` 0.0 0.0 (* _index 18.0)))))
    (bind _pathcost (`NavigationSystemV1.GetPathCost` (`self.K2_GetActorLocation` (`self.K2_GetPawn`)) _returnvalue null null))
    (if (and (!= _pathcost 0.0) (< _pathcost (`local.Path cost`)))
      (set `local.Loc` _returnvalue)
      (set `local.Path cost` _pathcost)))
  (return (`NavigationSystemV1.K2_GetRandomReachablePointInRadius` (`local.Loc`) 500.0 null null)))

(fn `Init`
  (bind _blackboard (`self.Blackboard`))
  (bind _asmatch_game_state (cast `MatchGameState` (`GameplayStatics.GetGameState`)))
  (bind _output_get (set `self.TargetDistance` (`MatchGameState.TargetDistance` _asmatch_game_state)))
  (`BlackboardComponent.SetValueAsFloat` _blackboard (`self.TargetDistanceKey`) _output_get)
  (`BlackboardComponent.SetValueAsObject` _blackboard (`self.EnemyActorKey`) null)
  (`BlackboardComponent.SetValueAsBool` _blackboard (`self.IsHaveBulletsKey`) true))

(fn `SetBullet`
  (locals (Koef :type "Array of Float (double-precision)"))
  (bind _returnvalue (`self.K2_GetPawn`))
  (bind _blackboard (`self.Blackboard`))
  (`/Engine/EditorBlueprintResources/StandardMacros.IsValid` _blackboard
    (:`Is Valid`
      (`/Engine/EditorBlueprintResources/StandardMacros.IsValid` _returnvalue
        (:`Is Valid`
          (bind _asdefault_character (cast `DefaultCharacter` (`BlackboardComponent.GetValueAsObject` _blackboard (`self.EnemyActorKey`))))
          (bind _asdefault_character_2 (cast `DefaultCharacter` _returnvalue))
          (bind _asmatch_game_state (cast `MatchGameState` (`GameplayStatics.GetGameState`)))
          (bind _returnvalue_2 (`KismetMathLibrary.VSize` (- (`self.K2_GetActorLocation` _asdefault_character) (`self.K2_GetActorLocation` _returnvalue))))
          (bind _returnvalue_3 (`KismetMathLibrary.Abs` (- _returnvalue_2 1500.0)))
          (bind _returnvalue_4 (`KismetMathLibrary.Abs` (- _returnvalue_2 1000.0)))
          (bind _returnvalue_5 (`KismetMathLibrary.Abs` (- _returnvalue_2 500.0)))
          (bind _returnvalue_6 (`KismetMathLibrary.FMax` _returnvalue_3 _returnvalue_4 _returnvalue_5))
          (bind _distancekoefforbullet (`MatchGameState.DistanceKoefForBullet` _asmatch_game_state))
          (bind _healthkoef (`MatchGameState.HealthKoef` _asmatch_game_state))
          (bind _returnvalue_7 (/ (+ (`DefaultCharacter.CurrentHealth` _asdefault_character_2) (`DefaultCharacter.Shield` _asdefault_character_2)) 200.0))
          (bind _returnvalue_8 (+ (* (- 1.0 (/ _returnvalue_3 _returnvalue_6)) _distancekoefforbullet) (* _healthkoef _returnvalue_7)))
          (bind _returnvalue_9 (* _healthkoef (/ (- 1.0 _returnvalue_7) 2.0)))
          (bind _returnvalue_10 (+ (* (- 1.0 (/ _returnvalue_4 _returnvalue_6)) _distancekoefforbullet) _returnvalue_9))
          (bind _returnvalue_11 (`KismetMathLibrary.FMax` _returnvalue_8 _returnvalue_10 (+ (* (- 1.0 (/ _returnvalue_5 _returnvalue_6)) _distancekoefforbullet) _returnvalue_9)))
          (bind _bulletmanager (`DefaultCharacter.BulletManager` _asdefault_character_2))
          (bind _countbullets (`BulletManagerComponent.CountBullets` _bulletmanager))
          (bind _returnvalue_12 (!= (`|GetArrayItem` _countbullets 1) 0))
          (bind _returnvalue_13 (!= (`|GetArrayItem` _countbullets 2) 0))
          (if (or (and (== _returnvalue_11 _returnvalue_8) (!= (`|GetArrayItem` _countbullets) 0)) (`KismetMathLibrary.BooleanNOR` _returnvalue_12 _returnvalue_13))
            (`BulletManagerComponent.SetCurrentBullet` _bulletmanager 0)
            (elif (or (and (== _returnvalue_11 _returnvalue_10) _returnvalue_12) (not _returnvalue_13))
              (`BulletManagerComponent.SetCurrentBullet` _bulletmanager 1)
              (else
                (`BulletManagerComponent.SetCurrentBullet` _bulletmanager 2)))))))))

(fn `SetFocal`
  (params (Delta :type "Float (double-precision)"))
  (bind _returnvalue (`self.GetControlRotation`))
  (bind _returnvalue_2 (`self.K2_GetPawn`))
  (bind _blackboard (`self.Blackboard`))
  (bind _returnvalue_3 (`BlackboardComponent.GetValueAsObject` _blackboard (`self.EnemyActorKey`)))
  (`KismetSystemLibrary.PrintString` (`KismetStringLibrary.Conv_DoubleToString` Delta))
  (`/Engine/EditorBlueprintResources/StandardMacros.IsValid` _blackboard
    (:`Is Valid`
      (`/Engine/EditorBlueprintResources/StandardMacros.IsValid` _returnvalue_3
        (:`Is Valid`
          (bind _asdefault_character (cast `DefaultCharacter` _returnvalue_3))
          (cast `DefaultCharacter` _returnvalue_2)
          (`self.K2_SetFocalPoint` (+ (`self.K2_GetActorLocation` _returnvalue_2) (`KismetMathLibrary.Conv_RotatorToVector` (`KismetMathLibrary.ComposeRotators` (* (`KismetMathLibrary.NormalizedDeltaRotator` (`KismetMathLibrary.Conv_VectorToRotator` (- (+ (`SceneComponent.K2_GetComponentLocation` (`Character.Mesh` _asdefault_character)) (0.0 0.0 20.0)) (`self.K2_GetActorLocation` _returnvalue_2))) (`KismetMathLibrary.Conv_VectorToRotator` (`KismetMathLibrary.GetForwardVector` _returnvalue))) (* Delta 10.0)) _returnvalue)))))
        (:`Is Not Valid`
          (`self.K2_ClearFocus`))))))

(fn `SetWeapon`
  (bind _returnvalue (`self.K2_GetPawn`))
  (bind _returnvalue_2 (`AIBlueprintHelperLibrary.GetBlackboard` null))
  (`/Engine/EditorBlueprintResources/StandardMacros.IsValid` _returnvalue_2
    (:`Is Valid`
      (`/Engine/EditorBlueprintResources/StandardMacros.IsValid` _returnvalue
        (:`Is Valid`
          (bind _asdefault_character (cast `DefaultCharacter` (`BlackboardComponent.GetValueAsObject` _returnvalue_2 (`self.EnemyActorKey`))))
          (bind _asmatch_game_state (cast `MatchGameState` (`GameplayStatics.GetGameState`)))
          (bind _asdefault_character_2 (cast `DefaultCharacter` (`self.K2_GetPawn`)))
          (bind (_bulletcolor _damage _speed _lineardamping _weaponkoef) (defaults `Object` (`BulletManagerComponent.CurrentBullet` (`DefaultCharacter.BulletManager` _asdefault_character_2))))
          (bind _bulletkoef (`MatchGameState.BulletKoef` _asmatch_game_state))
          (bind _distancekoefforweapon (`MatchGameState.DistanceKoefForWeapon` _asmatch_game_state))
          (bind _returnvalue_3 (`KismetMathLibrary.VSize` (- (`self.K2_GetActorLocation` _asdefault_character) (`self.K2_GetActorLocation` _returnvalue))))
          (bind _returnvalue_4 (`KismetMathLibrary.Abs` (- _returnvalue_3 1000.0)))
          (bind _returnvalue_5 (`KismetMathLibrary.Abs` (- _returnvalue_3 400.0)))
          (bind _returnvalue_6 (`KismetMathLibrary.Abs` (- _returnvalue_3 1500.0)))
          (bind _returnvalue_7 (`KismetMathLibrary.Abs` (- _returnvalue_3 600.0)))
          (bind _returnvalue_8 (`KismetMathLibrary.FMax` _returnvalue_4 _returnvalue_5 _returnvalue_6 _returnvalue_7))
          (bind _returnvalue_9 (+ (* (`|GetArrayItem` _weaponkoef) _bulletkoef) (* _distancekoefforweapon (- 1.0 (/ _returnvalue_4 _returnvalue_8)))))
          (bind _returnvalue_10 (+ (* (`|GetArrayItem` _weaponkoef 1) _bulletkoef) (* _distancekoefforweapon (- 1.0 (/ _returnvalue_5 _returnvalue_8)))))
          (bind _returnvalue_11 (+ (* (`|GetArrayItem` _weaponkoef 2) _bulletkoef) (* _distancekoefforweapon (- 1.0 (/ _returnvalue_6 _returnvalue_8)))))
          (bind _returnvalue_12 (`KismetMathLibrary.FMax` _returnvalue_9 _returnvalue_10 _returnvalue_11 (+ (* (`|GetArrayItem` _weaponkoef 3) _bulletkoef) (* _distancekoefforweapon (- 1.0 (/ _returnvalue_7 _returnvalue_8))))))
          (if (== _returnvalue_12 _returnvalue_9)
            (bind _weaponmanager (`DefaultCharacter.WeaponManager` _asdefault_character_2))
            (`WeaponManagerComponent.SetCurrentWeapon` _weaponmanager 0)
            (elif (== _returnvalue_12 _returnvalue_10)
              (`WeaponManagerComponent.SetCurrentWeapon` _weaponmanager 1)
              (elif (== _returnvalue_12 _returnvalue_11)
                (bind _indexweapon (`WeaponManagerComponent.IndexWeapon` _weaponmanager))
                (if (!= _indexweapon 2)
                  (`WeaponManagerComponent.SetCurrentWeapon` _weaponmanager 2)
                  (bind _asbow (cast `Bow` (`|GetArrayItem` (`WeaponManagerComponent.Weapons` _weaponmanager) _indexweapon)))
                  (`Bow.PressShoot` _asbow))
                (else
                  (`WeaponManagerComponent.SetCurrentWeapon` _weaponmanager 3))))))))))

(fn `UserConstructionScript`)