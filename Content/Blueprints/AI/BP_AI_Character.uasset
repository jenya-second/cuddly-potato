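; AI character Blueprint that exposes a function for changing its walk speed.
; UpdateSpeed writes the given value to the CharacterMovement component's MaxWalkSpeed, with no caller inside this Blueprint.
; BeginPlay and the construction script only call their parents, Possessed is empty, and Tick is disabled.
; Two debug prints, one showing a controller name, are left disconnected and never run.
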(event `self.ReceiveBeginPlay`
  (`parent.ReceiveBeginPlay`))

(event `self.ReceivePossessed`
  (params (NewController :type "Controller Object Reference")))

(fn `UpdateSpeed`
  (params (NewSpeed :type "Float (double-precision)"))
  (set `CharacterMovementComponent.MaxWalkSpeed` NewSpeed (`self.CharacterMovement`)))

(fn `UserConstructionScript`
  (`parent.UserConstructionScript`))