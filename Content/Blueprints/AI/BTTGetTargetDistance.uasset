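; Behavior tree task that keeps an AI's move location updated with a fight spot while it has line of sight.
; On execute it casts the owner to BP_AI_Controller and starts a looping short-interval timer.
; Each tick of the timer writes GetFightSpot's result to the PatrolLocationKey blackboard vector.
; When HasLineOfSightKey is false, it clears the timer and finishes successfully.
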(event `self.ReceiveExecuteAI`
  (params (OwnerController :type "AIController Object Reference") (ControlledPawn :type "Pawn Object Reference"))
  (bind _asbp_ai_controller (cast `/Game/Blueprints/AI/BP_AI_Controller` OwnerController))
  (bind _returnvalue (`KismetSystemLibrary.K2_SetTimerDelegate` (delegate `Find Location`) 0.1 true))
  (set `self.Timer` _returnvalue))

(event `Find Location`
  (bind _location (`/Game/Blueprints/AI/BP_AI_Controller.GetFightSpot` (stale `self.ReceiveExecuteAI` _asbp_ai_controller)))
  (bind _returnvalue (`AIBlueprintHelperLibrary.GetBlackboard` (stale `self.ReceiveExecuteAI` _asbp_ai_controller)))
  (`BlackboardComponent.SetValueAsVector` _returnvalue (`self.PatrolLocationKey`) _location)
  (if (not (`BlackboardComponent.GetValueAsBool` _returnvalue (`self.HasLineOfSightKey`)))
    (`KismetSystemLibrary.K2_ClearAndInvalidateTimerHandle` (`self.Timer`))
    (`self.FinishExecute` true)))