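; Behavior Tree task that makes an AI-controlled DefaultCharacter fire its currently selected weapon.
; It calls BotShoot on the WeaponManager's active weapon, then sums BulletManager's CountBullets to set the blackboard's has-bullets key.
; The task finishes successfully after a shot, but never calls FinishExecute when the cast fails or the weapon is invalid.
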(event `self.ReceiveExecuteAI`
  (params (OwnerController :type "AIController Object Reference") (ControlledPawn :type "Pawn Object Reference"))
  (bind _count (`self.Count`))
  (bind _asdefault_character (cast `DefaultCharacter` ControlledPawn))
  (bind _weaponmanager (`DefaultCharacter.WeaponManager` _asdefault_character))
  (bind _output (`|GetArrayItem` (`WeaponManagerComponent.Weapons` _weaponmanager) (`WeaponManagerComponent.IndexWeapon` _weaponmanager)))
  (`/Engine/EditorBlueprintResources/StandardMacros.IsValid` _output
    (:`Is Valid`
      (`DefaultWeapon.BotShoot` _output)
      (for _array_element (`BulletManagerComponent.CountBullets` (`DefaultCharacter.BulletManager` _asdefault_character))
        (set `self.Count` (+ _array_element _count)))
      (`BlackboardComponent.SetValueAsBool` (`AIBlueprintHelperLibrary.GetBlackboard` OwnerController) (`self.IsHaveBulletsKey`) (!= _count 0))
      (set `self.Count` 0)
      (`self.FinishExecute` true))))